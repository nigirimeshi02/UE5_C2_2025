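; Game mode that plays the game-clear and game-over cutscenes for the player.
; Each transition event waits briefly, then creates a Level Sequence player for its cutscene; game over also makes the player mesh visible first.
; A shared CreateBidingCutScene function binds the player character to the sequence and sets the instance-data transform origin to the player's transform, so playback is relative to the player's position.
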(event Custom|TransitionGameClear
  (Utilities|FlowControl|Delay 3.0)
  (bind (_outactor _returnvalue) (Sequencer|Player|CreateLevelSequencePlayer (Utilities|ResolveSoftReference (Variables|Default|GetGameClearCutScene))))
  (CallFunction|CreateBidingCutScene _outactor _returnvalue))

(event Custom|TransitionGameOver
  (Utilities|FlowControl|Delay 2.0)
  (bind _asbp_player (Utilities|Casting|CastToBP_Player (Game|GetPlayerCharacter 0)))
  (Rendering|SetVisibility (Variables|/Script/Engine.Character|GetMesh _asbp_player) true false)
  (bind (_outactor _returnvalue) (Sequencer|Player|CreateLevelSequencePlayer (Utilities|ResolveSoftReference (Variables|Default|GetGameOverCutScene))))
  (CallFunction|CreateBidingCutScene _outactor _returnvalue))

(event EventBeginPlay)

(event EventTick
  (params (DeltaSeconds :type Float%20%28single-precision%29)))

(fn ConstructionScript)

(fn CreateBidingCutScene
  (params (LevelSequenceActor :type Level%20Sequence%20Actor%20Object%20Reference) (LevelSequencePlayer :type Level%20Sequence%20Player%20Object%20Reference))
  (bind _returnvalue (Game|GetPlayerCharacter 0))
  (Variables|/Script/LevelSequence.LevelSequenceActor|SetbOverrideInstanceData LevelSequenceActor true)
  (bind _asdefault_level_sequence_instance_data (Utilities|Casting|CastToDefaultLevelSequenceInstanceData (Variables|/Script/LevelSequence.LevelSequenceActor|GetDefaultInstanceData LevelSequenceActor)))
  (Class|LevelSequenceActor|AddBinding LevelSequenceActor (|GetSequenceBinding) _returnvalue false)
  (Variables|/Script/LevelSequence.DefaultLevelSequenceInstanceData|SetTransformOrigin _asdefault_level_sequence_instance_data (Transformation|GetActorTransform _returnvalue))
  (Sequencer|Player|Play LevelSequencePlayer :!class /Script/MovieScene.MovieSceneSequencePlayer))