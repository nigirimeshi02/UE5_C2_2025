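; Player controller Blueprint that owns the player's health and stamina HUD widgets.
; On BeginPlay it creates WBP_Health and WBP_Stamina, stores references to them and adds both to the viewport.
; Two custom events take current and maximum health or stamina and pass the resulting ratio to the matching widget's update function.
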(event EventBeginPlay
  (Utilities|FlowControl|Sequence
    (:then_0
      (bind _returnvalue (UserInterface|CreateWidget "/Game/Game/UI/WBP_Health.WBP_Health_C"))
      (bind _output_get (Variables|Default|SetHealthRef _returnvalue))
      (UserInterface|Viewport|AddtoViewport _output_get 0))
    (:then_1
      (bind _returnvalue_2 (UserInterface|CreateWidget "/Game/Game/UI/WBP_Stamina.WBP_Stamina_C"))
      (bind _output_get_2 (Variables|Default|SetStaminaRef _returnvalue_2))
      (UserInterface|Viewport|AddtoViewport _output_get_2 0))))

(event EventTick
  (params (DeltaSeconds :type Float%20%28single-precision%29)))

(event EventUpdateHealthDisplay
  (params (Health :type Float%20%28double-precision%29) (MaxHealth :type Float%20%28double-precision%29))
  (Default|UpdateHealth (Variables|Default|GetHealthRef) (/ Health MaxHealth)))

(event EventUpdateStaminaDisplay
  (params (Stamina :type Float%20%28double-precision%29) (MaxStamina :type Float%20%28double-precision%29))
  (Default|UpdateStamina (Variables|Default|GetStaminaRef) (/ Stamina MaxStamina)))

(fn ConstructionScript)